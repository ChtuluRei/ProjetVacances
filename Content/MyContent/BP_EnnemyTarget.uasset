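; BP_EnnemyTarget is an enemy target that takes damage and shows its health on a healthbar widget.
; AnyDamage subtracts the incoming damage from HealthEnnemy, but the zero-health check leads to no action.
; Tick casts the HealthBarWidget's widget to WP_HealthbarEnnemy and sets its bar from health divided by 100, polling every frame rather than updating on damage.
; The HitByGrenade event is present but empty.
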(event Custom|HitByGrenade)

(event EventBeginPlay)

(event Collision|EventActorBeginOverlap
  (params (OtherActor :type Actor%20Object%20Reference)))

(event Game|Damage|EventAnyDamage
  (params (Damage :type Float%20%28single-precision%29) (DamageType :type Damage%20Type%20Object%20Reference) (InstigatedBy :type Controller%20Object%20Reference) (DamageCauser :type Actor%20Object%20Reference))
  (Variables|Default|SetHealthEnnemy (- (Variables|Default|GetHealthEnnemy) Damage))
  (if (<= (Variables|Default|GetHealthEnnemy) 0.0)
    _))

(event EventTick
  (params (DeltaSeconds :type Float%20%28single-precision%29))
  (bind _aswp_healthbar_ennemy (Utilities|Casting|CastToWP_HealthbarEnnemy (UserInterface|GetWidget (Variables|Default|GetHealthBarWidget))))
  (Progress|SetPercent (Variables|/Game/MyContent/WP_HealthbarEnnemy.WP_HealthbarEnnemy_C|GetHealthBarEnnemy _aswp_healthbar_ennemy) (/ (Variables|Default|GetHealthEnnemy) 1e+02)))

(fn ConstructionScript)