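; Timed grenade actor that explodes five seconds after BeginPlay, spawning an explosion particle and sound at its location.
; It then calls ApplyDamage with no target or amount set and runs a debug-drawn, single-hit sphere trace around itself.
; Only a BP_EnnemyTarget hit hides the Sphere1 component and destroys the grenade after a delay.
; Otherwise, it casts to BP_ThirdPersonCharacter with no further action.
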(event EventBeginPlay
  (bind _sphere (Variables|Default|GetSphere))
  (bind _returnvalue (Transformation|GetWorldLocation _sphere))
  ;[1 1 1] 5 secondes après avoir lancé la grenade, elle produira une particule d'explosion
  (Utilities|FlowControl|Delay 5.0)
  (Effects|SpawnEmitteratLocation "/Game/StarterContent/Particles/P_Explosion.P_Explosion" (Transformation|GetActorLocation))
  ;[1 1 1] Son de l'explosion
  (Audio|PlaySoundatLocation "/Game/StarterContent/Audio/Explosion_Cue.Explosion_Cue" (Transformation|GetActorLocation) "0, 0, 0" 1.0 1.0 0.0 0 0 0 0)
  (Game|Damage|ApplyDamage 0 0.0 0 0)
  (bind _outhit (Collision|SphereTraceByChannel _returnvalue _returnvalue 5e+02 "TraceTypeQuery1" true 0 "ForDuration"))
  ;[1 1 1] Pour faire disparaître la grenade un peu après l'explosion
  (Utilities|Casting|CastToBP_EnnemyTarget (.hitactor _outhit)
    (:then
      (Development|SetHiddeninGame (Variables|Default|GetSphere1) true false)
      (Utilities|FlowControl|Delay 3.0)
      (Actor|DestroyActor))
    (:CastFailed
      (Utilities|Casting|CastToBP_ThirdPersonCharacter (.hitactor _outhit)))))

(fn ConstructionScript)