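; BP_Platform is an elevator platform actor that moves when the third-person character enters its box trigger.
; Each overlap flips IsMovingUp and plays or reverses a timeline, which drives the Cube's relative Z location.
; The character's input is disabled when movement starts and re-enabled when the timeline finishes.
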(event OnComponentBeginOverlap(Box)
  (params (OverlappedComponent :type Primitive%20Component%20Object%20Reference) (OtherActor :type Actor%20Object%20Reference) (OtherComp :type Primitive%20Component%20Object%20Reference) (OtherBodyIndex :type Integer) (bFromSweep :type Boolean) (SweepResult :type Hit%20Result%20Structure%20%28by%20ref%29))
  (bind _asbp_third_person_character (Utilities|Casting|CastToBP_ThirdPersonCharacter OtherActor))
  (Variables|Default|SetAs%20BP%20Third%20Person%20Character _asbp_third_person_character)
  (if (Variables|Default|GetIsMovingUp?)
    (Variables|Default|SetIsMovingUp? false)
    (Input|DisableInput (Variables|Default|GetAs%20BP%20Third%20Person%20Character) 0)
    (bind _nouvelle_piste_0 (Timeline|Chronologie Reverse)
      (:Update
        (Transformation|SetRelativeLocation (Variables|Default|GetCube) (Math|Vector|MakeVector 0.0 0.0 _nouvelle_piste_0) false false))
      (:Finished
        (Input|EnableInput (Variables|Default|GetAs%20BP%20Third%20Person%20Character) 0)))
    (else
      (Variables|Default|SetIsMovingUp? true)
      (Input|DisableInput (Variables|Default|GetAs%20BP%20Third%20Person%20Character) 0)
      (Timeline|Chronologie Play))))

(event EventBeginPlay)

(event Collision|EventActorBeginOverlap
  (params (OtherActor :type Actor%20Object%20Reference)))

(event EventTick
  (params (DeltaSeconds :type Float%20%28single-precision%29)))

(fn ConstructionScript)